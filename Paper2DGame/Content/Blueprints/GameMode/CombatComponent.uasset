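; Combat component for a battle unit that runs its timed turn cycle and attack actions.
; A Haste-scaled timer requests turns from BattleGameMode; starting a party unit's turn opens its command HUD and orbits the dynamic camera around it.
; Melee attacks walk to the target via AI, play flipbook animations, return to the saved battle position, then end the turn and restart the timer.
; Ranged attack is an empty stub.
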(event `self.ReceiveBeginPlay`
  (bind _asbp_unit_base (cast `/Game/Blueprints/GameMode/BP_unitBase` (`self.GetOwner`)))
  (bind _output_get (set `self.UnitCharacter` _asbp_unit_base))
  (set `self.BattlePosition` (`Actor.GetTransform` _output_get))
  (`self.BeginBattle`))

(event `AttackCommand`
  (message `/Game/Blueprints/GameMode/BPI_DynamicCameraInterface.SetOrbit` (`Controller.GetViewTarget` (`GameplayStatics.GetPlayerController` 0)) false)
  (if (`self.IsRanged`)
    (`self.RangedAttack`)
    (else
      (`self.MeleeAttack`))))

(event `MeleeAttack`
  (bind _flipbook (`/Game/Blueprints/GameMode/BP_unitBase.Flipbook` (`self.UnitCharacter`)))
  (`|AIMoveTo` (`self.UnitCharacter`) (0.0 0.0 0.0) (`self.UnitTarget`) 100.0
    (:`then`
      (bind _actioncommandwindow (`self.ActionCommandWindow`)
        (:`then`
          (`Widget.RemoveFromParent` _actioncommandwindow)
          (`PaperFlipbookComponent.SetFlipbook` _flipbook (`self.WalkMontage`)))
        (:`else`)))
    (:`OnSuccess`
      (`PaperFlipbookComponent.SetFlipbook` _flipbook (`self.AttackMontage`))
      (`PaperFlipbookComponent.PlayFromStart` _flipbook)
      (`KismetSystemLibrary.Delay` (`PaperFlipbookComponent.GetFlipbookLength` _flipbook))
      (`PaperFlipbookComponent.SetFlipbook` _flipbook (`self.WalkMontage`))
      (`|AIMoveTo` (`self.UnitCharacter`) (.location (`self.BattlePosition`)) null
        (:`OnSuccess`
          (`PaperFlipbookComponent.SetFlipbook` _flipbook (`self.IdleMontage`))
          (`Actor.K2_SetActorRotation` (`self.UnitCharacter`) (.rotation (`self.BattlePosition`)) false)
          (`KismetSystemLibrary.Delay` 0.2)
          (`self.EndUnitTurn`))))))

(event `RangedAttack`)

(fn `BeginBattle`
  (bind _returnvalue (`KismetSystemLibrary.K2_SetTimer` self "RequestTurn" (+ (* (- 1.0 (`KismetMathLibrary.NormalizeToRange` (`self.Haste`) 0.0 255.0)) (- (`self.MaxActionTime`) (`self.MinActionTime`))) (`self.MinActionTime`))))
  (set `self.ActionTimer` _returnvalue))

(fn `EndUnitTurn`
  (`self.TurnEnded`)
  (`self.BeginBattle`))

(fn `RequestTurn`
  (bind _asbattle_game_mode (cast `/Game/Blueprints/GameMode/BattleGameMode` (`GameplayStatics.GetGameMode`)))
  (`/Game/Blueprints/GameMode/BattleGameMode.TurnRequest` _asbattle_game_mode (`self.UnitCharacter`)))

(fn `SetCamera`
  (bind _returnvalue (`GameplayStatics.GetActorOfClass` "/Game/Blueprints/GameMode/BP_DynamicCamera.BP_DynamicCamera_C"))
  (`PlayerController.SetViewTargetWithBlend` (`GameplayStatics.GetPlayerController` 0) _returnvalue 0.0 "VTBlend_Linear" 0.0 false)
  (message `/Game/Blueprints/GameMode/BPI_DynamicCameraInterface.SetDynamicLocation` _returnvalue (`self.UnitCharacter`) (0.0 0.0 0.0))
  (message `/Game/Blueprints/GameMode/BPI_DynamicCameraInterface.SetOrbit` (`Controller.GetViewTarget` (`GameplayStatics.GetPlayerController` 0)) true))

(fn `Start Unit Turn`
  (if (`KismetMathLibrary.ClassIsChildOf` (`GameplayStatics.GetObjectClass` (`self.UnitCharacter`)) "/Game/Blueprints/GameMode/PartyUnitBase.PartyUnitBase_C")
    (bind _returnvalue (`|CreateWidget` "/Game/Blueprints/GameMode/UI/Widgets/UnitBattleHud.UnitBattleHud_C" null (`self.UnitCharacter`)))
    (bind _output_get (set `self.ActionCommandWindow` _returnvalue))
    (`UserWidget.AddToViewport` _output_get 0)
    (`self.SetCamera`)))