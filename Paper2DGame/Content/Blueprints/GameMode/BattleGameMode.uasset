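; Battle game mode that sets up a turn-based fight and runs its turn queue.
; On BeginPlay it switches to a top-down camera, gathers party and enemy units, then adds party units to the battle HUD after a short delay.
; Units request turns into a unique queue; a DoOnce gate lets one combat component act at a time, binds its turn-ended event, and reopens when readying the next turn.
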(event `self.ReceiveBeginPlay`
  (bind _returnvalue (`GameplayStatics.GetActorOfClass` "/Game/Blueprints/GameMode/Camera_TopDown.Camera_TopDown_C"))
  (bind _output_get (set `self.MainBattleCamera` _returnvalue))
  (`PlayerController.SetViewTargetWithBlend` (`GameplayStatics.GetPlayerController` 0) _output_get 0.0 "VTBlend_Linear" 0.0 false)
  (bind _outactors (`GameplayStatics.GetAllActorsOfClass` "/Game/Blueprints/GameMode/PartyUnitBase.PartyUnitBase_C"))
  (set `self.PartyUnits` _outactors)
  (bind _outactors_2 (`GameplayStatics.GetAllActorsOfClass` "/Game/Blueprints/GameMode/EnemyUnitBase.EnemyUnitBase_C"))
  (set `self.EnemyUnits` _outactors_2)
  (`KismetSystemLibrary.Delay` 0.2)
  (bind _asbattle_player_controller (cast `/Game/Blueprints/GameMode/BattlePlayerController` (`GameplayStatics.GetPlayerController` 0)))
  (set `self.Battle Hud` (`/Game/Blueprints/GameMode/BattlePlayerController.BattleHud` _asbattle_player_controller))
  (for _array_element (`self.PartyUnits`)
    (`/Game/Blueprints/GameMode/UI/Widgets/BattleHeadUpDisplay.AddPartyUnitToHud` (`self.Battle Hud`) _array_element)))

(event `TurnRequest`
  (params (Unit :type "/Game/Blueprints/GameMode/BP_unitBase Object Reference"))
  (`KismetArrayLibrary.Array_AddUnique` (`self.TurnOrder`) Unit)
  (`self.StartTurn`))

(event `StartTurn`
  (bind _combatcomponent (`/Game/Blueprints/GameMode/BP_unitBase.CombatComponent` (`|GetArrayItem` (`self.TurnOrder`))))
  (`/Engine/EditorBlueprintResources/StandardMacros.DoOnce` false :!label _label
    (:`Completed`
      (if (`KismetArrayLibrary.Array_IsValidIndex` (`self.TurnOrder`))
        (`/Game/Blueprints/GameMode/CombatComponent.Start Unit Turn` _combatcomponent)
        (add `/Game/Blueprints/GameMode/CombatComponent.TurnEnded` _combatcomponent (`|CreateDelegate` :!event `ReadyNextTurn`))
        (`KismetArrayLibrary.Array_Remove` (`self.TurnOrder`))
        (else
          (`self.ReadyNextTurn`))))))

(event `ReadyNextTurn`
  (`|ExecutionSequence`
    (:`then_0`
      (goto _label :!via `Reset`))
    (:`then_1`
      (if (`KismetArrayLibrary.Array_IsValidIndex` (`self.TurnOrder`))
        (`self.StartTurn`)))))

(fn `UserConstructionScript`)