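; BP_DynamicCamera is a spring-arm camera actor that can follow an actor, glide to a location, or orbit.
; SetDynamicLocation snaps and attaches it to a valid actor while keeping world rotation, otherwise storing a target location.
; Tick interpolates toward that target only while the camera is unattached.
; SetOrbit toggles RotatingMovement and spring-arm yaw inheritance, resetting actor rotation when orbiting stops.
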(event `/Game/Blueprints/GameMode/BPI_DynamicCameraInterface.SetOrbit`
  (params (IsOrbiting :type Boolean))
  (set `RotatingMovementComponent.RotationRate` (`KismetMathLibrary.SelectRotator` (struct :`Yaw` 10.0) (struct) IsOrbiting) (`self.RotatingMovement`))
  (bind _output_get (set `SpringArmComponent.bInheritYaw` IsOrbiting (`self.SpringArm`)))
  (if (not _output_get)
    (`self.K2_SetActorRotation` (struct))))

(event `/Game/Blueprints/GameMode/BPI_DynamicCameraInterface.SetDynamicLocation`
  (params (Actor :type "Actor Object Reference") (Vector :type "Vector Structure"))
  (`/Engine/EditorBlueprintResources/StandardMacros.IsValid` Actor
    (:`Is Valid`
      (`self.K2_AttachToActor` Actor "None" "SnapToTarget" "KeepWorld" "KeepWorld")
      (`SceneComponent.K2_SetRelativeRotation` :`self` (`self.Camera`)))
    (:`Is Not Valid`
      (set `self.TargetLocation` Vector))))

(event `self.ReceiveTick`
  (params (DeltaSeconds :type "Float (single-precision)"))
  (`/Engine/EditorBlueprintResources/StandardMacros.IsValid` (`self.GetAttachParentActor`)
    (:`Is Not Valid`
      (`self.K2_SetActorLocation` (`KismetMathLibrary.VInterpTo` (`self.K2_GetActorLocation`) (`self.TargetLocation`) DeltaSeconds 5.0)))))

(fn `UserConstructionScript`)